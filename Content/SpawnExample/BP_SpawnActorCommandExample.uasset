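; BP_SpawnActorCommandExample is an example undoable command that spawns an actor and records it in a state object.
; Do runs the parent logic, then stores the spawned actor in State at the command's Index.
; Undo runs the parent logic, then clears that slot in State.
; The SpawnActor override simply passes through the parent's result.
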(event `self.Do`
  (`parent.Do`)
  (`/CommandPlugin/SpawnExample/BP_SpawnState.SetSpawnedActorAt` (`self.State`) (`self.Index`) (`self.GetSpawnedActor`)))

(event `self.Undo`
  (`parent.Undo`)
  (`/CommandPlugin/SpawnExample/BP_SpawnState.SetSpawnedActorAt` (`self.State`) (`self.Index`) null))

(fn `SpawnActor`
  (returns (ReturnValue :type "Actor Object Reference"))
  (bind _returnvalue (`parent.SpawnActor`))
  (return _returnvalue))