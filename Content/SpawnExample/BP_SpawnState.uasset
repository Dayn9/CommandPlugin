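; BP_SpawnState is a state Blueprint for a spawn example that tracks actors spawned into ten indexed slots.
; Init sizes the SpawnedActor array, a getter reads a slot, and the setter writes one and then calls OnStateUpdated to signal the change.
; IndexToTransform maps a slot index to a position in an Offset-spaced row centered on the Y axis and raised by Offset on Z.
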(event `Init`
  (`KismetArrayLibrary.Array_Resize` (`self.SpawnedActor`) 10))

(fn `GetSpawnedActorAt`
  (params (Index :type Integer))
  (returns (SpawnedActor :type "Actor Object Reference"))
  (return (`|GetArrayItem` (`self.SpawnedActor`) Index)))

(fn `IndexToTransform`
  (params (Index :type Integer))
  (returns (ReturnValue :type "Transform Structure"))
  (bind _offset (`self.Offset`))
  (return (`KismetMathLibrary.Conv_VectorToTransform` (`KismetMathLibrary.MakeVector` 0.0 (+ (* Index _offset -1.0) (* _offset 4.5)) (`self.Offset`)))))

(fn `SetSpawnedActorAt`
  (params (Index :type Integer) (SpawnedActor :type "Actor Object Reference"))
  (`KismetArrayLibrary.Array_Set` (`self.SpawnedActor`) Index SpawnedActor)
  (`self.OnStateUpdated`))