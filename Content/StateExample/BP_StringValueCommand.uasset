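; BP_StringValueCommand is a command Blueprint in the state example that sets a string value on a State object.
; Do writes NextValue to the State through SetStringValue, and GetDisplayString labels the command with that value.
; Undo makes the same call with NextValue, so it does not restore a previous value.
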(event `self.Do`
  (`/CommandPlugin/StateExample/BP_ExampleState.SetStringValue` (`self.State`) (`self.NextValue`)))

(event `self.Undo`
  (`/CommandPlugin/StateExample/BP_ExampleState.SetStringValue` (`self.State`) (`self.NextValue`)))

(fn `GetDisplayString`
  (returns (ReturnValue :type String))
  (return (`KismetStringLibrary.Concat_StrStr` "Set String: " (`self.NextValue`))))