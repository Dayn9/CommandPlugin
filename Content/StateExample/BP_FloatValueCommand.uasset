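; BP_FloatValueCommand is an undoable command that sets a float value on a State object.
; Do and Undo both call FlipValue, which swaps the stored Value with the state's current float, so one operation serves both directions.
; GetDisplayString returns a "Set Float:" label followed by the state's current float value.
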(event `self.Do`
  (`self.FlipValue` :!label _label))

(event `self.Undo`
  (goto _label))

(fn `FlipValue`
  (locals (Temp :type "Float (double-precision)" :default 0.0))
  (set `local.Temp` (`/CommandPlugin/StateExample/BP_ExampleState.GetFloatValue` (`self.State`)))
  (`/CommandPlugin/StateExample/BP_ExampleState.SetFloatValue` (`self.State`) (`self.Value`))
  (set `self.Value` (`local.Temp`)))

(fn `GetDisplayString`
  (returns (ReturnValue :type String))
  (return (`KismetStringLibrary.Concat_StrStr` "Set Float: " (`KismetStringLibrary.Conv_DoubleToString` (`/CommandPlugin/StateExample/BP_ExampleState.GetFloatValue` (`self.State`))))))