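; BP_ExampleState is an example state container that holds a string value and a float value.
; Each value has a getter and a setter.
; Both setters store the new value and then call OnStateUpdated to signal the change, without checking whether the value differs.
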(fn `GetFloatValue`
  (returns (FloatValue :type "Float (double-precision)"))
  (return (`self.FloatValue`)))

(fn `GetStringValue`
  (returns (StringValue :type String))
  (return (`self.StringValue`)))

(fn `SetFloatValue`
  (params (FloatValue :type "Float (double-precision)"))
  (set `self.FloatValue` FloatValue)
  (`self.OnStateUpdated`) ; Trigger state change updates
)

(fn `SetStringValue`
  (params (StringValue :type String))
  (set `self.StringValue` StringValue)
  (`self.OnStateUpdated`) ; Trigger state change updates
)